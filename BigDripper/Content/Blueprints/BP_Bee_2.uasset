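; Bee swarm actor that shows six bee components flying out along world Y and back, then vanishing.
; Spawn makes the bees visible; BeginPlay and Hide conceal them, reset the timer and turn them around.
; While visible and the game instance's GameRun is set, Tick moves them for two seconds, then ReturnBee flips and reverses them until Hide at four.
; Movement is a fixed per-frame step, so distance depends on frame rate.
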(event `self.ReceiveBeginPlay`
  (`self.Hide`))

(event `self.ReceiveTick`
  (params (DeltaSeconds :type "Float (single-precision)"))
  (bind _asinstance (cast `/Game/Blueprints/Instance` (`GameplayStatics.GetGameInstance`)))
  (if (== (`/Game/Blueprints/Instance.GameRun` _asinstance) true)
    (if (`self.Visible`)
      (`self.MoveBees`)
      (bind _output_get (set `self.Time` (+ (`self.Time`) DeltaSeconds)))
      (if (>= _output_get 4.0)
        (`self.Hide`)
        (elif (> (`self.Time`) 2.0)
          _)))))

(fn `Hide`
  (`SceneComponent.SetVisibility` (`self.Bee`) false false)
  (`SceneComponent.SetVisibility` (`self.Bee1`) false false)
  (`SceneComponent.SetVisibility` (`self.Bee2`) false false)
  (`SceneComponent.SetVisibility` (`self.Bee4`) false false)
  (`SceneComponent.SetVisibility` (`self.Bee5`) false false)
  (`SceneComponent.SetVisibility` (`self.Bee3`) false false)
  (set `self.Visible` false)
  (set `self.Time` 0.0)
  (`SceneComponent.K2_SetWorldRotation` (`self.Bee`) (struct :`Yaw` 180.0) false false)
  (`SceneComponent.K2_SetWorldRotation` (`self.Bee1`) (struct :`Yaw` 180.0) false false)
  (`SceneComponent.K2_SetWorldRotation` (`self.Bee2`) (struct :`Yaw` 180.0) false false)
  (`SceneComponent.K2_SetWorldRotation` (`self.Bee3`) (struct :`Yaw` 180.0) false false)
  (`SceneComponent.K2_SetWorldRotation` (`self.Bee4`) (struct :`Yaw` 180.0) false false)
  (`SceneComponent.K2_SetWorldRotation` (`self.Bee5`) (struct :`Yaw` 180.0) false false))

(fn `MoveBees`
  (bind _bee1 (`self.Bee1`))
  (bind _bee2 (`self.Bee2`))
  (bind _bee3 (`self.Bee3`))
  (bind _bee4 (`self.Bee4`))
  (bind _bee5 (`self.Bee5`))
  (bind _bee (`self.Bee`))
  (bind (_returnvalue_x _returnvalue_y _returnvalue_z) (`KismetMathLibrary.BreakVector` (`SceneComponent.K2_GetComponentLocation` _bee2)))
  (bind (_returnvalue_x_2 _returnvalue_y_2 _returnvalue_z_2) (`KismetMathLibrary.BreakVector` (`SceneComponent.K2_GetComponentLocation` _bee3)))
  (bind (_returnvalue_x_3 _returnvalue_y_3 _returnvalue_z_3) (`KismetMathLibrary.BreakVector` (`SceneComponent.K2_GetComponentLocation` _bee4)))
  (bind (_returnvalue_x_4 _returnvalue_y_4 _returnvalue_z_4) (`KismetMathLibrary.BreakVector` (`SceneComponent.K2_GetComponentLocation` _bee5)))
  (bind (_returnvalue_x_5 _returnvalue_y_5 _returnvalue_z_5) (`KismetMathLibrary.BreakVector` (`SceneComponent.K2_GetComponentLocation` _bee)))
  (bind (_returnvalue_x_6 _returnvalue_y_6 _returnvalue_z_6) (`KismetMathLibrary.BreakVector` (`SceneComponent.K2_GetComponentLocation` _bee1)))
  (if (>= (`self.Time`) 2.0)
    (`self.ReturnBee`)
    (else
      (`SceneComponent.K2_SetWorldLocation` _bee1 (`KismetMathLibrary.MakeVector` _returnvalue_x_6 (+ _returnvalue_y_6 -5.0) _returnvalue_z_6) false false)
      (`SceneComponent.K2_SetWorldLocation` _bee2 (`KismetMathLibrary.MakeVector` _returnvalue_x (+ _returnvalue_y -5.0) _returnvalue_z) false false)
      (`SceneComponent.K2_SetWorldLocation` _bee3 (`KismetMathLibrary.MakeVector` _returnvalue_x_2 (+ _returnvalue_y_2 -5.0) _returnvalue_z_2) false false)
      (`SceneComponent.K2_SetWorldLocation` _bee4 (`KismetMathLibrary.MakeVector` _returnvalue_x_3 (+ _returnvalue_y_3 -5.0) _returnvalue_z_3) false false)
      (`SceneComponent.K2_SetWorldLocation` _bee5 (`KismetMathLibrary.MakeVector` _returnvalue_x_4 (+ _returnvalue_y_4 -5.0) _returnvalue_z_4) false false)
      (`SceneComponent.K2_SetWorldLocation` _bee (`KismetMathLibrary.MakeVector` _returnvalue_x_5 (+ _returnvalue_y_5 -5.0) _returnvalue_z_5) false false))))

(fn `ReturnBee`
  (bind _bee1 (`self.Bee1`))
  (bind _bee2 (`self.Bee2`))
  (bind _bee3 (`self.Bee3`))
  (bind _bee4 (`self.Bee4`))
  (bind _bee5 (`self.Bee5`))
  (bind _bee (`self.Bee`))
  (bind (_returnvalue_x _returnvalue_y _returnvalue_z) (`KismetMathLibrary.BreakVector` (`SceneComponent.K2_GetComponentLocation` _bee2)))
  (bind (_returnvalue_x_2 _returnvalue_y_2 _returnvalue_z_2) (`KismetMathLibrary.BreakVector` (`SceneComponent.K2_GetComponentLocation` _bee3)))
  (bind (_returnvalue_x_3 _returnvalue_y_3 _returnvalue_z_3) (`KismetMathLibrary.BreakVector` (`SceneComponent.K2_GetComponentLocation` _bee4)))
  (bind (_returnvalue_x_4 _returnvalue_y_4 _returnvalue_z_4) (`KismetMathLibrary.BreakVector` (`SceneComponent.K2_GetComponentLocation` _bee5)))
  (bind (_returnvalue_x_5 _returnvalue_y_5 _returnvalue_z_5) (`KismetMathLibrary.BreakVector` (`SceneComponent.K2_GetComponentLocation` _bee)))
  (bind (_returnvalue_x_6 _returnvalue_y_6 _returnvalue_z_6) (`KismetMathLibrary.BreakVector` (`SceneComponent.K2_GetComponentLocation` _bee1)))
  (`SceneComponent.K2_SetWorldRotation` :`self` _bee1)
  (`SceneComponent.K2_SetWorldLocation` _bee1 (`KismetMathLibrary.MakeVector` _returnvalue_x_6 (+ _returnvalue_y_6 5.0) _returnvalue_z_6) false false)
  (`SceneComponent.K2_SetWorldRotation` :`self` _bee2)
  (`SceneComponent.K2_SetWorldLocation` _bee2 (`KismetMathLibrary.MakeVector` _returnvalue_x (+ _returnvalue_y 5.0) _returnvalue_z) false false)
  (`SceneComponent.K2_SetWorldRotation` :`self` _bee3)
  (`SceneComponent.K2_SetWorldLocation` _bee3 (`KismetMathLibrary.MakeVector` _returnvalue_x_2 (+ _returnvalue_y_2 5.0) _returnvalue_z_2) false false)
  (`SceneComponent.K2_SetWorldRotation` :`self` _bee4)
  (`SceneComponent.K2_SetWorldLocation` _bee4 (`KismetMathLibrary.MakeVector` _returnvalue_x_3 (+ _returnvalue_y_3 5.0) _returnvalue_z_3) false false)
  (`SceneComponent.K2_SetWorldRotation` :`self` _bee5)
  (`SceneComponent.K2_SetWorldLocation` _bee5 (`KismetMathLibrary.MakeVector` _returnvalue_x_4 (+ _returnvalue_y_4 5.0) _returnvalue_z_4) false false)
  (`SceneComponent.K2_SetWorldRotation` :`self` _bee)
  (`SceneComponent.K2_SetWorldLocation` _bee (`KismetMathLibrary.MakeVector` _returnvalue_x_5 (+ _returnvalue_y_5 5.0) _returnvalue_z_5) false false))

(fn `Spawn`
  (`SceneComponent.SetVisibility` (`self.Bee`) true false)
  (`SceneComponent.SetVisibility` (`self.Bee1`) true false)
  (`SceneComponent.SetVisibility` (`self.Bee2`) true false)
  (`SceneComponent.SetVisibility` (`self.Bee3`) true false)
  (`SceneComponent.SetVisibility` (`self.Bee4`) true false)
  (`SceneComponent.SetVisibility` (`self.Bee5`) true false)
  (set `self.Visible` true))

(fn `UserConstructionScript`)